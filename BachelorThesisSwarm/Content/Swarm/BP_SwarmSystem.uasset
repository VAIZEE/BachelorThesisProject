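; Actor that drives a Niagara particle swarm for an nDisplay CAVE simulation.
; Construction and BeginPlay push particle count, bounds, neighbor-grid settings, debug flags and the CAVE center point into the Niagara system.
; Each tick it emits a primary-only cluster event carrying delta time and controller rotation, which the listener feeds into Niagara to keep nodes in sync.
; It registers as the particle readback handler, though the callback does nothing with the data.
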(event EventBeginPlay
  ;[1 1 1] Initialize on Begin Play
  (CallFunction|InitializeSwarmSystem)
  (Class|DisplayClusterBlueprintAPI|AddClusterEventListener (Class|DisplayClusterBlueprintLib|GetAPI) self)
  (Class|NiagaraComponent|SetVariableBool (Variables|Default|GetNiagaraSwarmSystem) "InCaveSimulation" true))

(event Collision|EventActorBeginOverlap
  (params (OtherActor :type Actor%20Object%20Reference)))

(event EventTick
  (params (DeltaSeconds :type Float%20%28single-precision%29))
  ;[1 1 1] Comment
  (bind _returnvalue (Actor|GetActorOfClass "/Game/Swarm/BP_Controller.BP_Controller_C"))
  (Class|DisplayClusterBlueprintAPI|EmitClusterEventJson (Class|DisplayClusterBlueprintLib|GetAPI) (Utilities|Struct|MakeDisplayClusterClusterEventJson "SyncPrimaryNodeData" "" "" (Utilities|Map|MakeMap "PrimaryDeltaTime" (Utilities|String|ToString(Float) DeltaSeconds) "PrimaryNodeControllerRotation" (Utilities|String|ToString(Vector) (Math|Vector|MakeVector (.Roll (Math|Rotator|BreakRotator (Transformation|GetWorldRotation (Variables|/Game/Swarm/BP_Controller.BP_Controller_C|GetCube _returnvalue)))) (.Pitch (Math|Rotator|BreakRotator (Transformation|GetWorldRotation (Variables|/Game/Swarm/BP_Controller.BP_Controller_C|GetCube _returnvalue)))) (.Yaw (Math|Rotator|BreakRotator (Transformation|GetWorldRotation (Variables|/Game/Swarm/BP_Controller.BP_Controller_C|GetCube _returnvalue)))))))) true))

(event EventEndPlay
  (params (EndPlayReason :type EEndPlayReason%20Enum :default "Destroyed"))
  ;[1 1 1] Remove Cluster Event Listener
  (Class|DisplayClusterBlueprintAPI|RemoveClusterEventListener (Class|DisplayClusterBlueprintLib|GetAPI) self))

(event EventOnClusterEventJson
  (params (Event :type Display%20Cluster%20Cluster%20Event%20Json%20Structure%20%28by%20ref%29))
  (bind (_name _type _category _parameters) (Utilities|Struct|BreakDisplayClusterClusterEventJson Event))
  ;[1 1 1] Handle incoming Cluster Event
  (if (Utilities|Enum|Equal(Enum) _name "SyncPrimaryNodeData")
    (Effects|Components|ParticleSystem|SetFloatParameter (Variables|Default|GetNiagaraSwarmSystem) "PrimaryNodeDeltaTime" (Math|Conversions|ToFloat(Integer) (.Value (Utilities|Map|Find _parameters "PrimaryDeltaTime"))))
    (Niagara|SetNiagaraVariable(Vector3) (Variables|Default|GetNiagaraSwarmSystem) "ControllerRotation" (.OutConvertedVector (Math|Conversions|ToVector(Float) (.Value (Utilities|Map|Find _parameters "PrimaryNodeControllerRotation")))))))

(event EventParticleData
  (params (Data :type Array%20of%20Basic%20Particle%20Data%20Structures) (NiagaraSystem :type Niagara%20System%20Object%20Reference) (SimulationPositionOffset :type Vector%20%28by%20ref%29 :default "0, 0, 0"))
  ;[1 1 1] Event for Particle Data Readback
  (for _array_element Data
    _))

(fn ConstructionScript
  (CallFunction|InitializeSwarmSystem))

(fn InitializeSwarmSystem
  (bind _niagaraswarmsystem (Variables|Default|GetNiagaraSwarmSystem))
  (bind _boundshight (Variables|SwarmSettings|GetBoundsHight))
  (bind _boundswidth (Variables|SwarmSettings|GetBoundsWidth))
  (bind _neighborgridcellsinwidth (Variables|NeighborGridSettings|GetNeighborGridCellsInWidth))
  (bind _returnvalue (Math|Vector|MakeVector _boundswidth _boundswidth _boundshight))
  (Utilities|IsValid _niagaraswarmsystem
    (:Is%20Valid
      ;[1 1 1] Set Particle Count
      (Class|NiagaraComponent|SetVariableInt _niagaraswarmsystem "ParticleCount" (Variables|SwarmSettings|GetParticleCount))
      ;[1 1 1] Set System and Grid Bounds
      (Niagara|SetNiagaraVariable(Vector3) _niagaraswarmsystem "GridSize" _returnvalue)
      (Class|NiagaraComponent|SetSystemFixedBounds _niagaraswarmsystem (Math|Box|MakeBox (* _returnvalue -0.5) (* _returnvalue 0.5)))
      ;[1 1 1] Set Neighbor Grid Parameters
      (Class|NiagaraComponent|SetVariableInt _niagaraswarmsystem "CellsSizeX" _neighborgridcellsinwidth)
      (Class|NiagaraComponent|SetVariableInt _niagaraswarmsystem "CellsSizeY" _neighborgridcellsinwidth)
      (Class|NiagaraComponent|SetVariableInt _niagaraswarmsystem "CellsSizeZ" (Variables|NeighborGridSettings|GetNeighborGridCellsInHight))
      (Class|NiagaraComponent|SetVariableInt _niagaraswarmsystem "MaxNeighborCount" (Variables|NeighborGridSettings|GetNeigborGridMaxParticlesPerCell))
      (Effects|Components|ParticleSystem|SetBoolParameter _niagaraswarmsystem "ShowDebugGrid" (Variables|NeighborGridSettings|GetShowDebugGrid))
      (Effects|Components|ParticleSystem|SetVectorParameter _niagaraswarmsystem "GridCenter" (Transformation|GetWorldLocation (Variables|Default|GetNiagaraSwarmSystem)))
      ;[1 1 1] Add user Position
      (bind _returnvalue_2 (Actor|GetActorOfClass "/Game/FHWedelCaveTemplate/NDC_FHWedelCave.NDC_FHWedelCave_C"))
      (Class|NiagaraDataInterfaceArrayFunctionLibrary|SetNiagaraArrayVector _niagaraswarmsystem "UserDefinedPoints" (Utilities|Array|MakeArray (Transformation|GetWorldLocation (Variables|/Game/FHWedelCaveTemplate/NDC_FHWedelCave.NDC_FHWedelCave_C|Getcave_center _returnvalue_2))))
      (Effects|Components|ParticleSystem|SetFloatParameter _niagaraswarmsystem "UserDefinedPointsRadius" (Variables|SwarmSettings|GetUserDefinedPointsRadius))
      ;[1 1 1] Set Show Target Direction
      (Class|NiagaraComponent|SetVariableBool _niagaraswarmsystem "ShowDebugTargetDirection" (Variables|SwarmSettings|GetShowDebugTargetDirection))
      ;[1 1 1] Set Cast Shadows
      (Rendering|SetCastShadow _niagaraswarmsystem (Variables|SwarmSettings|GetCastShadows))
      ;[1 1 1] Set Callback handler for Particle data Readback
      (Class|NiagaraComponent|SetVariableObject (Variables|Default|GetNiagaraSwarmSystem) "BPCallbackHandler" self))))